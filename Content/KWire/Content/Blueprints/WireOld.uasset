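; WireOld is a Blueprint for a wire that displays a three-state signal by changing its material.
; Every Tick it compares the Output string against TRUE, FALSE and OFF and sets the matching material on the first slot of the Wire component.
; It polls rather than reacting to changes, and nothing in this Blueprint writes Output.
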(event `self.ReceiveTick`
  (params (DeltaSeconds :type "Float (single-precision)"))
  (bind _output (`self.Output`))
  (bind _wire (`self.Wire`))
  (if (`KismetStringLibrary.EqualEqual_StrStr` _output "TRUE")
    (`PrimitiveComponent.SetMaterial` _wire 0 "/Game/Materials/glow2.glow2")
    (elif (`KismetStringLibrary.EqualEqual_StrStr` _output "FALSE")
      (`PrimitiveComponent.SetMaterial` _wire 0 "/Game/Materials/Bench_01_Masked.Bench_01_Masked")
      (elif (`KismetStringLibrary.EqualEqual_StrStr` _output "OFF")
        (`PrimitiveComponent.SetMaterial` _wire 0 "/Game/Props/Materials/M_MaterialSphere_Plain.M_MaterialSphere_Plain")))))

(fn `UserConstructionScript`)