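; Or_Gun_Pickup is a gun pickup actor that spins in place and removes itself when an actor overlaps it.
; On BeginPlay a timeline adds one degree of yaw to the GunModelHere component on each update, so the spin rate depends on frame rate.
; Any overlap destroys the actor after a very short delay, with no filtering or weapon-granting logic in this Blueprint.
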(event `self.ReceiveActorBeginOverlap`
  (params (OtherActor :type "Actor Object Reference"))
  (`KismetSystemLibrary.Delay` 0.001)
  (`self.K2_DestroyActor`))

(event `self.ReceiveBeginPlay`
  (`Timeline|Timeline_0`
    (:`Update`
      (bind _returnvalue (`SceneComponent.GetRelativeTransform` (`self.Gun Model Here`)))
      (`SceneComponent.SetRelativeTransform` (`self.Gun Model Here`) (`KismetMathLibrary.MakeTransform` (.location _returnvalue) (`KismetMathLibrary.MakeRot` (.pitch (.rotation _returnvalue)) (+ (.yaw (.rotation _returnvalue)) 1.0) (.roll (.rotation _returnvalue))) (.scale _returnvalue)) false))))

(fn `NewFunction_0`)

(fn `UserConstructionScript`)