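; Logic gate panel for a circuit puzzle that becomes AND, OR or XOR, or is cleared, when hit by projectiles identified by display-name prefix.
; Each change swaps the visible gate mesh and, unless the panel is static, re-evaluates input wire states.
; Output wires go dead without a gate or with any OFF input, otherwise turn on or off by gate logic, then propagate downstream.
; The Inverted NAND/NOR branches are unconnected.
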(event EventHit
  (params (MyComp :type Primitive%20Component%20Object%20Reference) (Other :type Actor%20Object%20Reference) (OtherComp :type Primitive%20Component%20Object%20Reference) (bSelfMoved :type Boolean) (HitLocation :type Vector :default "0, 0, 0") (HitNormal :type Vector :default "0, 0, 0") (NormalImpulse :type Vector :default "0, 0, 0") (Hit :type Hit%20Result%20Structure%20%28by%20ref%29))
  (bind _returnvalue (Utilities|GetDisplayName Other))
  (bind _returnvalue_2 (Utilities|String|GetSubstring _returnvalue 0 12))
  (CallFunction|InvisifyAll)
  (if (Utilities|Enum|Equal(Enum) _returnvalue_2 "ProjectileAN")
    (Variables|Default|SetGateType "and")
    (Effects|SpawnEmitteratLocation "/Game/Particles/P_Explosion.P_Explosion" HitLocation)
    (Audio|PlaySoundatLocation "/Game/Android/Sounds/MetalSlice.MetalSlice" HitLocation)
    (Rendering|SetVisibility (Variables|Default|Getand) true false)
    ;[1 1 1] When hit, update outgoing wires
    (CallFunction|Update :!label _label)
    (elif (Utilities|Enum|Equal(Enum) _returnvalue_2 "ProjectileOR")
      (Variables|Default|SetGateType "or")
      (Effects|SpawnEmitteratLocation "/Game/Particles/P_Explosion.P_Explosion" HitLocation)
      (Audio|PlaySoundatLocation "/Game/Android/Sounds/MetalSlice.MetalSlice" HitLocation)
      (Rendering|SetVisibility (Variables|Default|Getor) true false)
      (goto _label)
      (elif (Utilities|Enum|Equal(Enum) _returnvalue_2 "ProjectileXO")
        (Variables|Default|SetGateType "xor")
        (Effects|SpawnEmitteratLocation "/Game/Particles/P_Explosion.P_Explosion" "0, 0, 0")
        (Audio|PlaySoundatLocation "/Game/Android/Sounds/MetalSlice.MetalSlice" "0, 0, 0")
        (Rendering|SetVisibility (Variables|Default|GetXOR) true false)
        (goto _label)
        (elif (Utilities|Enum|Equal(Enum) _returnvalue_2 "ProjectileCL")
          (Variables|Default|SetGateType "none")
          (Audio|PlaySoundatLocation "/Game/Android/Sounds/Button.Button" "0, 0, 0")
          (goto _label))))))

(event EventBeginPlay
  (CallFunction|InvisifyAll)
  (if (Utilities|Enum|Equal(Enum) (Variables|Default|GetGateType) "and")
    (Rendering|SetVisibility (Variables|Default|Getand) true false)
    (elif (Utilities|Enum|Equal(Enum) (Variables|Default|GetGateType) "or")
      (Rendering|SetVisibility (Variables|Default|Getor) true false)
      (elif (Utilities|Enum|Equal(Enum) (Variables|Default|GetGateType) "xor")
        (Rendering|SetVisibility (Variables|Default|GetXOR) true false)
        (elif (Utilities|Enum|Equal(Enum) (Variables|Default|GetGateType) "none")
          _
          (else
            _)))))
  ;[1 1 1] When hit, update outgoing wires
  (CallFunction|Update))

(fn ConstructionScript)

(fn Update
  (if (not (Variables|Default|GetIsStatic))
    ;[1 1 1] If any wires aren't flowing, cut off flow
    (if (Utilities|Enum|Equal(Enum) (Variables|Default|GetGateType) "none")
      (Default|TurnDead (Variables|Default|GetOutput_Wires) :!label _label)
      ;[1 1 1] Propogate Changes Further along circuit
      (for _array_element (Variables|Default|GetOutput_Wires) :!label _label_2
        (Default|UpdateConnected _array_element))
      (else
        (bind _contains_ (CallFunction|ContainsState (Variables|Default|GetInput_Wires) (Variables|Default|GetOFF)))
        (if _contains_
          (goto _label)
          (elif (Utilities|Enum|Equal(Enum) (Variables|Default|GetGateType) "and")
            ;[1 1 1] If AND Contains False,Output False
            (bind _contains__2 (CallFunction|ContainsState (Variables|Default|GetInput_Wires) (Variables|Default|GetFALSE)))
            (if _contains__2
              ;[1 1 1] Update Outgoing Wires
              (Default|TurnOff (Variables|Default|GetOutput_Wires) :!label _label_3)
              (goto _label_2)
              (else
                (Default|Turnon (Variables|Default|GetOutput_Wires) :!label _label_4)
                (goto _label_2)))
            (elif (Utilities|Enum|Equal(Enum) (Variables|Default|GetGateType) "or")
              ;[1 1 1] If OR Contains True, Output True
              (bind _contains__3 (CallFunction|ContainsState (Variables|Default|GetInput_Wires) (Variables|Default|GetTRUE)))
              (if _contains__3
                (goto _label_4)
                (else
                  (goto _label_3)))
              (elif (Utilities|Enum|Equal(Enum) (Variables|Default|GetGateType) "xor")
                (bind _contains__4 (CallFunction|ContainsState (Variables|Default|GetInput_Wires) (Variables|Default|GetFALSE)))
                (if _contains__4
                  (bind _contains__5 (CallFunction|ContainsState (Variables|Default|GetInput_Wires) (Variables|Default|GetTRUE)))
                  (if _contains__5
                    (goto _label_4)
                    (else
                      (goto _label_3)))
                  (else
                    (goto _label_3)))))))))))

(fn ContainsState
  (params (Input_Wires :type Array%20of%20Wire%202%20Object%20References) (State :type String))
  (LocalVariables|SetFound false)
  (bind _array_element (Utilities|Array|ForEachLoopwithBreak Input_Wires :!label _label)
    (:LoopBody
      (bind _state (Default|GetState _array_element))
      (if (Utilities|Enum|Equal(Enum) _state State)
        (LocalVariables|SetFound true)
        (goto _label Break)))
    (:Completed
      (return (LocalVariables|GetFound)))))

(fn InvisifyAll
  (Rendering|SetVisibility (Variables|Default|Getand) false false)
  (Rendering|SetVisibility (Variables|Default|Getor) false false)
  (Rendering|SetVisibility (Variables|Default|GetXOR) false false))