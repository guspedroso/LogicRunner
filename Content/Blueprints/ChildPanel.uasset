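; ChildPanel is a child Blueprint of a panel with four wire inputs and four wire outputs.
; Its construction script runs the parent's script, then checks each wire reference and sets a matching valid flag for those that are assigned.
; The flags are only ever set to true here, and the script does nothing else with the wires.
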(fn `UserConstructionScript`
  (`parent.UserConstructionScript`)
  (`|ExecutionSequence`
    (:`then_0`
      (`self.IsValid` (`self.Wire_In_01`)
        (:`IsValid`
          (set `self.Wire01Valid` true))))
    (:`then_1`
      (`self.IsValid` (`self.Wire_In_02`)
        (:`IsValid`
          (set `self.Wire02Valid` true))))
    (:`then_2`
      (`self.IsValid` (`self.Wire_In_03`)
        (:`IsValid`
          (set `self.Wire03Valid` true))))
    (:`then_3`
      (`self.IsValid` (`self.Wire_In_04`)
        (:`IsValid`
          (set `self.Wire04Valid` true))))
    (:`then_4`
      (`self.IsValid` (`self.WireOut_01`)
        (:`IsValid`
          (set `self.WireOut_01_Valid` true))))
    (:`then_5`
      (`self.IsValid` (`self.WireOut_02`)
        (:`IsValid`
          (set `self.WireOut_02_Valid` true))))
    (:`then_6`
      (`self.IsValid` (`self.WireOut_03`)
        (:`IsValid`
          (set `self.WireOut_03_Valid` true))))
    (:`then_7`
      (`self.IsValid` (`self.WireOut_04`)
        (:`IsValid`
          (set `self.WireOut_04_Valid` true))))))