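; A holding Blueprint of logic copied from a level Blueprint, driving a boolean-logic puzzle with doors and deadly fire, with most object references unresolved.
; BeginPlay seeds gate inputs and outputs as "TRUE"/"FALSE" strings.
; Actor hit handlers relay outputs after a short delay to play or reverse animations.
; Tick polls outputs to drive more animations, toggle FireDeadly and its paired effects, and feed downstream gate inputs.
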(event `OnActorHit_None_Copy`
  (params (SelfActor :type "Actor Object Reference") (OtherActor :type "Actor Object Reference") (NormalImpulse :type "Object.Vector Structure") (Hit :type "EngineTypes.HitResult Structure (by ref)"))
  (bind _output (`/Game/Blueprints/LogicPanel.Output` ""))
  ;[1 1 1] Door Opening
  (`KismetSystemLibrary.Delay` 0.2)
  (set `/Game/KWire/Content/Blueprints/WireOld.Output` _output "")
  (if (`KismetStringLibrary.EqualEqual_StrStr` _output "TRUE")
    (`MatineeActor.Play` "")
    (else
      (`MatineeActor.Reverse` ""))))

(event `self.ReceiveBeginPlay`
  (set `/Game/Blueprints/LogicPanel.Inputs` (`|MakeArray` "TRUE" "TRUE") "")
  (set `/Game/Blueprints/LogicPanel.Inputs` (`|MakeArray` "FALSE" "TRUE") "")
  (set `/Game/Blueprints/LogicPanel.Inputs` (`|MakeArray` "TRUE" "TRUE") "")
  (set `/Game/Blueprints/LogicPanel.Inputs` (`|MakeArray` "TRUE" "FALSE") "")
  (set `/Game/Blueprints/LogicPanel.Inputs` (`|MakeArray` "FALSE" "TRUE") "")
  (set `/Game/Blueprints/LogicPanel.Inputs` (`|MakeArray` "TRUE" "FALSE" "TRUE") "")
  (set `/Game/KWire/Content/Blueprints/WireOld.Output` "TRUE" "")
  (set `/Game/KWire/Content/Blueprints/WireOld.Output` "TRUE" "")
  (set `/Game/KWire/Content/Blueprints/WireOld.Output` "FALSE" "")
  (set `/Game/KWire/Content/Blueprints/WireOld.Output` "TRUE" ""))

(event `OnActorHit_None_Copy`
  (params (SelfActor :type "Actor Object Reference") (OtherActor :type "Actor Object Reference") (NormalImpulse :type "Object.Vector Structure") (Hit :type "EngineTypes.HitResult Structure (by ref)"))
  (bind _output (`/Game/Blueprints/LogicPanel.Output` ""))
  ;[1 1 1] Door Opening
  (`KismetSystemLibrary.Delay` 0.2)
  (set `/Game/KWire/Content/Blueprints/WireOld.Output` _output "")
  (if (`KismetStringLibrary.EqualEqual_StrStr` _output "TRUE")
    (`MatineeActor.Play` "")
    (else
      (`MatineeActor.Reverse` ""))))

(event `self.ReceiveTick`
  (params (DeltaSeconds :type "Float (single-precision)"))
  (bind _output (`/Game/Blueprints/LogicPanel.Output` ""))
  ;[1 1 1] Door Opening
  (if (`KismetStringLibrary.EqualEqual_StrStr` (`/Game/Blueprints/LogicPanel.Output` "") "TRUE")
    (`MatineeActor.Play` "")
    (else
      (`MatineeActor.Reverse` "")))
  (if (`KismetStringLibrary.EqualEqual_StrStr` (`/Game/Blueprints/LogicPanel.Output` "") "TRUE")
    (`MatineeActor.Play` "")
    (else
      (`MatineeActor.Reverse` "")))
  (if (`KismetStringLibrary.EqualEqual_StrStr` (`/Game/Blueprints/LogicPanel.Output` "") "TRUE")
    (`MatineeActor.Reverse` "")
    (if (`KismetStringLibrary.EqualEqual_StrStr` _output "TRUE") :!label _label
      (set `self.FireDeadly` false)
      (`ActorComponent.Deactivate` "")
      (`ActorComponent.Deactivate` "")
      (else
        (set `self.FireDeadly` true)
        (`ActorComponent.Activate` "" false)
        (`ActorComponent.Activate` "" false)))
    (set `/Game/Blueprints/LogicPanel.Inputs` (`|MakeArray` (`/Game/Blueprints/LogicPanel.Output` "") _output) "")
    (if (`KismetStringLibrary.EqualEqual_StrStr` (`/Game/Blueprints/LogicPanel.Output` "") "TRUE")
      (`MatineeActor.Play` "")
      (else
        (`MatineeActor.Reverse` "")))
    (elif (and (== false false) (== false true))
      (`MatineeActor.Play` "")
      (goto _label))))

(fn `UserConstructionScript`)