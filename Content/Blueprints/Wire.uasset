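; Wire Blueprint that acts as a switchable link, showing a live or dead state and relaying it to an output actor.
; The Wireon and WireOff events set the Live flag, swap the WireMesh material and send the matching on/off message to OutputActor when it is valid.
; The construction script applies the material for the current Live value, so the initial state is visible on placement.
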(event `self.Wire_on`
  (bind _outputactor (`self.OutputActor`))
  (set `self.bLive` true)
  (`PrimitiveComponent.SetMaterial` (`self.WireMesh`) 0 "/Game/Materials/WireOnMat.WireOnMat")
  (`/Engine/EditorBlueprintResources/StandardMacros.IsValid` _outputactor
    (:`Is Valid`
      (message `/Game/Blueprints/WireInterface.Wire_on` _outputactor))))

(event `self.Wire_Off`
  (bind _outputactor (`self.OutputActor`))
  (set `self.bLive` false)
  (`PrimitiveComponent.SetMaterial` (`self.WireMesh`) 0 "/Game/Materials/WireOffMat.WireOffMat")
  (`/Engine/EditorBlueprintResources/StandardMacros.IsValid` _outputactor
    (:`Is Valid`
      (message `/Game/Blueprints/WireInterface.Wire_Off` _outputactor))))

(fn `UserConstructionScript`
  (if (`self.bLive`)
    (`PrimitiveComponent.SetMaterial` (`self.WireMesh`) 0 "/Game/Materials/WireOnMat.WireOnMat")
    (else
      (`PrimitiveComponent.SetMaterial` (`self.WireMesh`) 0 "/Game/Materials/WireOffMat.WireOffMat"))))