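; Logic gate panel Blueprint that computes a boolean Output from an Inputs array as either an AND or an OR gate.
; Every Tick evaluates the current GateType: AND is true unless any input is false, OR is true if any input is true.
; Projectile hits switch the gate type by matching the first 12 characters of the other actor's display name to "ProjectileAN" or "ProjectileOR".
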(event `self.ReceiveTick`
  (params (DeltaSeconds :type "Float (single-precision)"))
  (if (== (`self.GateType`) "and")
    ;[1 1 1] If AND Contains False,Output False
    (if (`KismetArrayLibrary.Array_Contains` (`self.Inputs`) false)
      (set `self.Output` false)
      (else
        (set `self.Output` true)))
    (elif (== (`self.GateType`) "or")
      ;[1 1 1] If OR Contains True, Output True
      (set `self.Output` (`KismetArrayLibrary.Array_Contains` (`self.Inputs`) true)))))

(event `self.ReceiveHit`
  (params (MyComp :type "PrimitiveComponent Object Reference") (Other :type "Actor Object Reference") (OtherComp :type "PrimitiveComponent Object Reference") (bSelfMoved :type Boolean) (HitLocation :type "Object.Vector Structure") (HitNormal :type "Object.Vector Structure") (NormalImpulse :type "Object.Vector Structure") (Hit :type "EngineTypes.HitResult Structure (by ref)"))
  (bind _returnvalue (`KismetStringLibrary.GetSubstring` (`KismetSystemLibrary.GetDisplayName` Other) 0 12))
  (if (`KismetStringLibrary.EqualEqual_StrStr` _returnvalue "ProjectileAN")
    (set `self.GateType` "and")
    (elif (`KismetStringLibrary.EqualEqual_StrStr` _returnvalue "ProjectileOR")
      (set `self.GateType` "or"))))

(fn `UserConstructionScript`)