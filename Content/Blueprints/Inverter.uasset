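; Inverter is a logic gate actor that drives its Output to the opposite of its Input.
; Update reads the Input's three-valued state: TRUE turns the Output off, FALSE turns it on, and OFF turns it dead.
; The event graph and construction script are empty, so the gate changes only when Update is called.
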(event `self.ReceiveBeginPlay`)

(event `self.ReceiveActorBeginOverlap`
  (params (OtherActor :type "Actor Object Reference")))

(event `self.ReceiveTick`
  (params (DeltaSeconds :type "Float (single-precision)")))

(fn `Update`
  (bind _state (`self.Get_State` (`self.Input`)))
  (if (== _state "OFF")
    (`self.Turn_Dead` (`self.Output`))
    (elif (== _state "TRUE")
      (`self.Turn_Off` (`self.Output`))
      (elif (== _state "FALSE")
        (`self.Turn On` (`self.Output`))))))

(fn `UserConstructionScript`)