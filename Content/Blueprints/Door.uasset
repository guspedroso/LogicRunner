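; Door Blueprint that opens or closes through a Matinee sequence in response to wire on and off events.
; Wireon reverses the Matinee and activates two fire effects, while WireOff plays the Matinee forward and deactivates them.
; Both events act only when both Fire1 and Fire2 references are valid, so the Matinee does not move without them.
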(event `self.Wire_on`
  (bind _fire1 (`self.Fire1`))
  (`/Engine/EditorBlueprintResources/StandardMacros.IsValid` _fire1
    (:`Is Valid`
      (`/Engine/EditorBlueprintResources/StandardMacros.IsValid` (`self.Fire2`)
        (:`Is Valid`
          (`MatineeActor.Reverse` (`self.Matinee`))
          (`ActorComponent.Activate` _fire1 false)
          (`ActorComponent.Activate` (`self.Fire2`) false))))))

(event `self.Wire_Off`
  (bind _fire1 (`self.Fire1`))
  (`/Engine/EditorBlueprintResources/StandardMacros.IsValid` _fire1
    (:`Is Valid`
      (`/Engine/EditorBlueprintResources/StandardMacros.IsValid` (`self.Fire2`)
        (:`Is Valid`
          (`MatineeActor.Play` (`self.Matinee`))
          (`ActorComponent.Deactivate` _fire1)
          (`ActorComponent.Deactivate` (`self.Fire2`)))))))

(fn `UserConstructionScript`)