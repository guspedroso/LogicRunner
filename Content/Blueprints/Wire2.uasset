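; Wire2 is a circuit wire with three states (on, off and unpowered), each shown by its own material on the wire mesh.
; TurnOn, TurnOff and TurnDead set the state, fire WireOn or WireOff, then propagate through UpdateConnected to OutputObjects.
; Panels and inverters update themselves, chained wires copy the state recursively, and other devices receive on/off messages.
; The construction script previews the initial state, BeginPlay applies it, and GetState reports it.
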(event EventBeginPlay
  (if (Variables|Default|GetisPowered)
    (if (Variables|Default|GetbLive)
      (CallFunction|Turnon)
      (else
        (CallFunction|TurnOff)))
    (else
      (CallFunction|TurnDead))))

(fn ConstructionScript
  (if (Variables|Default|GetisPowered)
    (if (Variables|Default|GetbLive)
      (Rendering|Material|SetMaterial (Variables|Default|GetWireMesh) 0 "/Game/Materials/WireOnMat.WireOnMat")
      (else
        (Rendering|Material|SetMaterial (Variables|Default|GetWireMesh) 0 "/Game/Materials/WireOffMat.WireOffMat")))
    (else
      (Rendering|Material|SetMaterial (Variables|Default|GetWireMesh) 0 "/Game/Android/Materials/white_emissive.white_emissive"))))

(fn GetState
  (if (Variables|Default|GetisPowered)
    (if (Variables|Default|GetbLive)
      (LocalVariables|Setreturn_val "TRUE")
      (else
        (LocalVariables|Setreturn_val "FALSE")))
    (else
      (LocalVariables|Setreturn_val "OFF")))
  (return (LocalVariables|Getreturn_val)))

(fn Turnon
  (Variables|Default|SetisPowered true)
  (Variables|Default|SetbLive true)
  (Rendering|Material|SetMaterial (Variables|Default|GetWireMesh) 0 "/Game/Materials/WireOnMat.WireOnMat")
  (CallFunction|Wireon)
  (CallFunction|UpdateConnected))

(fn TurnOff
  (Variables|Default|SetisPowered true)
  (Variables|Default|SetbLive false)
  (Rendering|Material|SetMaterial (Variables|Default|GetWireMesh) 0 "/Game/Materials/WireOffMat.WireOffMat")
  (CallFunction|WireOff)
  (CallFunction|UpdateConnected))

(fn TurnDead
  (Variables|Default|SetisPowered false)
  (Rendering|Material|SetMaterial (Variables|Default|GetWireMesh) 0 "/Game/Android/Materials/white_emissive.white_emissive")
  (CallFunction|WireOff)
  (CallFunction|UpdateConnected))

(fn UpdateConnected
  (for _array_element (Variables|Default|GetOutput%20Objects)
    ;[1 1 1] Connected Object is Panel
    (bind _aspanel_v3 (Utilities|Casting|CastToPanelV3 _array_element)
      (:then
        (Default|Update _aspanel_v3))
      (:CastFailed
        (bind _asinverter (Utilities|Casting|CastToInverter _array_element)
          (:then
            (Default|Update _asinverter))
          (:CastFailed
            ;[1 1 1] Connected Object is another wire
            (bind _aswire_2 (Utilities|Casting|CastToWire2 _array_element)
              (:then
                (if (Variables|Default|GetisPowered)
                  (if (Variables|Default|GetbLive)
                    (CallFunction|Turnon _aswire_2)
                    (else
                      (CallFunction|TurnOff _aswire_2)))
                  (else
                    (CallFunction|TurnDead _aswire_2))))
              (:CastFailed
                ;[1 1 1] Connected Object is a device
                (if (and (Variables|Default|GetbLive) (Variables|Default|GetisPowered))
                  (Class|WireInterface|Wireon(Message) _array_element)
                  (else
                    (Class|WireInterface|WireOff(Message) _array_element)))))))))))