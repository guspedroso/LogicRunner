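; A logic gate panel whose gate type the player sets by hitting it with projectiles.
; Hit reads the projectile's display name prefix to set AND, OR or none and swap the panel material, adding an explosion when a gate is placed.
; Tick derives a three-state Output from Inputs: OFF when any input is off or no gate is set, otherwise the gate result, with Inverted giving NAND and NOR.
; An XOR check exists but is unconnected.
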(event `self.ReceiveTick`
  (params (DeltaSeconds :type "Float (single-precision)"))
  ;[1 1 1] If any wires aren't flowing, cut off flow
  (if (`KismetArrayLibrary.Array_Contains` (`self.Inputs`) (`self.OFF`))
    (set `self.Output` (`self.OFF`) :!label _label)
    (elif (== (`self.GateType`) "none")
      (goto _label)
      (elif (== (`self.GateType`) "and")
        ;[1 1 1] If AND Contains False,Output False
        (if (`KismetArrayLibrary.Array_Contains` (`self.Inputs`) (`self.FALSE`))
          ;[1 1 1] Inverted handles NAND and NOR
          (if (`self.inverted`) :!label _label_2
            (set `self.Output` (`self.TRUE`) :!label _label_3)
            (else
              (set `self.Output` (`self.FALSE`) :!label _label_4)))
          (else
            (if (`self.inverted`) :!label _label_5
              (goto _label_4)
              (else
                (goto _label_3)))))
        (elif (== (`self.GateType`) "or")
          ;[1 1 1] If OR Contains True, Output True
          (if (`KismetArrayLibrary.Array_Contains` (`self.Inputs`) (`self.TRUE`))
            (goto _label_5)
            (else
              (goto _label_2))))))))

(event `self.ReceiveHit`
  (params (MyComp :type "PrimitiveComponent Object Reference") (Other :type "Actor Object Reference") (OtherComp :type "PrimitiveComponent Object Reference") (bSelfMoved :type Boolean) (HitLocation :type "Object.Vector Structure") (HitNormal :type "Object.Vector Structure") (NormalImpulse :type "Object.Vector Structure") (Hit :type "EngineTypes.HitResult Structure (by ref)"))
  (bind _returnvalue (`KismetStringLibrary.GetSubstring` (`KismetSystemLibrary.GetDisplayName` Other) 0 12))
  (if (`KismetStringLibrary.EqualEqual_StrStr` _returnvalue "ProjectileAN")
    (set `self.GateType` "and")
    (`GameplayStatics.SpawnEmitterAtLocation` "/Game/Particles/P_Explosion.P_Explosion" HitLocation)
    (`PrimitiveComponent.SetMaterial` (`self.StaticMesh1`) 0 "/Game/Materials/M_ProjectileAND.M_ProjectileAND")
    (`KismetSystemLibrary.PrintString` "AND Placed!")
    (elif (`KismetStringLibrary.EqualEqual_StrStr` _returnvalue "ProjectileOR")
      (set `self.GateType` "or")
      (`GameplayStatics.SpawnEmitterAtLocation` "/Game/Particles/P_Explosion.P_Explosion" HitLocation)
      (`PrimitiveComponent.SetMaterial` (`self.StaticMesh1`) 0 "/Game/Materials/M_ProjectileOR.M_ProjectileOR")
      (`KismetSystemLibrary.PrintString` "OR Placed!")
      (elif (`KismetStringLibrary.EqualEqual_StrStr` _returnvalue "ProjectileCL")
        (set `self.GateType` "none")
        (`PrimitiveComponent.SetMaterial` (`self.StaticMesh1`) 0 "/Game/Android/Materials/FloorWhite.FloorWhite")))))

(fn `NewFunction_0`
  (params (NewParam :type "Actor Class Reference")))

(fn `UserConstructionScript`)