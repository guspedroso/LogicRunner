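; FireKillBox is a fire hazard that kills the player on contact until it is switched off.
; When the player character overlaps the Collider while KillSwitch is true, it destroys the character and opens Example_Map.
; The Wireon event disarms the hazard by clearing KillSwitch and hiding the Fire component and its children.
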(event `self.Collider.OnComponentBeginOverlap`
  (params (OtherActor :type "Actor Object Reference") (OtherComp :type "PrimitiveComponent Object Reference") (OtherBodyIndex :type Integer) (bFromSweep :type Boolean) (SweepResult :type "EngineTypes.HitResult Structure (by ref)"))
  ;[1 1 1] Zombie/Fire Attack
  (if (== (`GameplayStatics.GetPlayerCharacter` 0) OtherActor)
    (if (`self.KillSwitch`)
      (`self.K2_DestroyActor` (`GameplayStatics.GetPlayerCharacter` 0))
      (`GameplayStatics.OpenLevel` "Example_Map"))))

(event `self.Wire_on`
  (set `self.KillSwitch` false)
  (`SceneComponent.SetHiddenInGame` (`self.Fire`) true true))

(fn `UserConstructionScript`)