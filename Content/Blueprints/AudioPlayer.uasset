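; AudioPlayer is a wire-triggered Blueprint that plays a sound attached to its Box1 component.
; Wireon plays AudioWhenActivated the first time it fires, with the ActHasPlayed flag blocking repeats.
; WireOff has the same one-shot guard through DeactHasPlayed, but its play call has no sound assigned, leaving AudioWhenDeactivated unused.
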(event `self.Wire_on`
  (if (not (`self.Act Has Played`))
    (`GameplayStatics.PlaySoundAttached` (`self.Audio When Activated`) (`self.Box1`))
    (set `self.Act Has Played` true)))

(event `self.Wire_Off`
  (if (not (`self.Deact Has Played`))
    (`GameplayStatics.PlaySoundAttached` null (`self.Box1`))
    (set `self.Deact Has Played` true)))

(fn `UserConstructionScript`)