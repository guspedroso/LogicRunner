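; NewHUD is a HUD Blueprint that draws a crosshair texture near the middle of the screen.
; On each DrawHUD it reads player 0's viewport size and draws a square sized by CrossSize.
; The top-left sits a quarter of CrossSize before the midpoint, so the image is slightly off-centre toward bottom-right.
; It also prints a debug "Hello" every draw, and the construction script is empty.
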(event `self.ReceiveDrawHUD`
  (params (SizeX :type Integer) (SizeY :type Integer))
  (bind _crosssize (`self.CrossSize`))
  (bind (_sizex _sizey) (`PlayerController.GetViewportSize` (`GameplayStatics.GetPlayerController` 0)))
  (bind _returnvalue (`KismetMathLibrary.Conv_IntToDouble` _crosssize))
  (bind _returnvalue_2 (* _crosssize -0.5))
  (`self.DrawTexture` (`self.Croshair`) (* (+ _returnvalue_2 (`KismetMathLibrary.Conv_IntToDouble` _sizex)) 0.5) (* (+ _returnvalue_2 (`KismetMathLibrary.Conv_IntToDouble` _sizey)) 0.5) _returnvalue _returnvalue 0.0 0.0 1.0 1.0)
  (`KismetSystemLibrary.PrintString` "Hello"))

(fn `UserConstructionScript`)